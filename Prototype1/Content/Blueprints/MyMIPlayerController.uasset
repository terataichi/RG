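; Player controller that holds the player's money and inventory of purchased weapons and Arch actors.
; Buy events deduct money, recording weapon entries or spawning Arch actors at a set location.
; Server-prefixed events cycle the selected Arch by mouse wheel, rotate it in yaw steps by middle click, remove it from the list without destroying it, or take one back.
; U, J and Q are debug keys for money and weapon listing.
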(event `Key|U`
  (params (Key :type "Key Structure"))
  (:`Pressed`
    (`self.AddMoneyCE` 99999)))

(event `Key|J`
  (params (Key :type "Key Structure"))
  (:`Pressed`
    (`self.SubMoneyCE` 1000000)))

(event `Key|Q`
  (params (Key :type "Key Structure"))
  (:`Pressed`
    (for _array_element (`self.MyWeaponList`)
      (`KismetSystemLibrary.PrintString` (`KismetSystemLibrary.GetDisplayName` _array_element)))))

(event `AddMoneyCE`
  (params (Value :type Integer))
  (set `self.Money` (+ (`self.Money`) Value)))

(event `SubMoneyCE`
  (params (Value :type Integer))
  (set `self.Money` (- (`self.Money`) Value)))

(event `BuyWeaponEV`
  (params (Weapon :type "/Game/Blueprints/Weapons/BP_WeaponBase Object Reference") (Value :type Integer))
  (`self.BuyWeapon` Weapon Value))

(event `BuyArchEV`
  (params (value :type Integer) (ArchClass :type "/Game/Stage/BP/StageObj/BP_ArchBase Class Reference"))
  (`self.Buy Arch` value ArchClass))

(event `Key|MouseScrollUp`
  (params (Key :type "Key Structure"))
  (:`Pressed`
    (`self.ServerChangeArchTarget` true)
    (`self.ServerSetArchRatation` :!label _label)))

(event `Key|MouseScrollDown`
  (params (Key :type "Key Structure"))
  (:`Pressed`
    (`self.ServerChangeArchTarget` false)
    (goto _label)))

(event `Key|MiddleMouseButton`
  (params (Key :type "Key Structure"))
  (:`Pressed`
    (`self.ServerAddAngle`)
    (goto _label)))

(event `ServerChangeArchTarget`
  (params (IsIncrement :type Boolean))
  (`self.ChangeArchTargetNum` IsIncrement)
  (`self.ClampArchTargetNum`)
  (`KismetSystemLibrary.PrintString` (`KismetStringLibrary.Conv_IntToString` (`self.ArchTargetNum`))))

(event `ServerRemoveItem`
  (`self.DeleteArch`))

(event `ServerTakeArch`
  (params (Actor :type "Actor Object Reference (by ref)"))
  (`self.TakeArch` Actor))

(event `ServerAddAngle`
  (bind _output_get (set `self.ArchAngle` (+ (`self.ArchAngle`) 90.0)))
  (if (> _output_get 360.0)
    (set `self.ArchAngle` 0.0)))

(event `ServerSetArchRatation`
  (bind _output (`|GetArrayItem` (`self.MyArchList`) (`self.ArchTargetNum`)))
  (if (`KismetSystemLibrary.IsValid` _output)
    (`self.K2_SetActorRotation` _output (`KismetMathLibrary.MakeRotator` 0.0 0.0 (`self.ArchAngle`)) true)))

(fn `Buy Arch`
  (params (Value :type Integer) (ArchClass :type "/Game/Stage/BP/StageObj/BP_ArchBase Class Reference"))
  (bind _returnvalue (`|SpawnActorFromClass` ArchClass (`KismetMathLibrary.MakeTransform` (`self.Spawn Transform Location`)) "AlwaysSpawn" "OverrideRootScale" null null))
  (`KismetArrayLibrary.Array_Add` (`self.MyArchList`) _returnvalue)
  (`self.SubMoneyCE` Value))

(fn `BuyWeapon`
  (params (weapon :type "/Game/Blueprints/Weapons/BP_WeaponBase Object Reference") (value :type Integer))
  (`KismetArrayLibrary.Array_Add` (`self.MyWeaponList`) weapon)
  (`self.SubMoneyCE` value))

(fn `ChangeArchTargetNum`
  (params (isIncrement :type Boolean))
  (if isIncrement
    (bind _result (`/Engine/EditorBlueprintResources/StandardMacros.IncrementInt` (`self.ArchTargetNum`))
      (:`  `
        (bind _output_get (set `self.ArchTargetNum` _result))
        (if (>= _output_get (`KismetArrayLibrary.Array_Length` (`self.MyArchList`)))
          (set `self.ArchTargetNum` 0))))
    (else
      (bind _result_2 (`/Engine/EditorBlueprintResources/StandardMacros.DecrementInt` (`self.ArchTargetNum`))
        (:`  `
          (bind _output_get_2 (set `self.ArchTargetNum` _result_2))
          (if (< _output_get_2 0)
            (set `self.ArchTargetNum` (- (`KismetArrayLibrary.Array_Length` (`self.MyArchList`)) 1))))))))

(fn `ClampArchTargetNum`
  (set `self.ArchTargetNum` (`KismetMathLibrary.Clamp` (`self.ArchTargetNum`) 0 (`KismetArrayLibrary.Array_Length` (`self.MyArchList`)))))

(fn `DeleteArch`
  (`KismetArrayLibrary.Array_Remove` (`self.MyArchList`) (`self.ArchTargetNum`)))

(fn `GetArchTarget`
  (returns (Arch :type "/Game/Stage/BP/StageObj/BP_ArchBase Object Reference"))
  (return (`|GetArrayItem` (`self.MyArchList`) (`self.ArchTargetNum`))))

(fn `TakeArch`
  (params (Actor :type "Actor Object Reference (by ref)"))
  (bind _asbp_arch_base (cast `/Game/Stage/BP/StageObj/BP_ArchBase` Actor))
  (`self.K2_SetActorLocation` _asbp_arch_base (`self.Spawn Transform Location`) false true)
  (`KismetArrayLibrary.Array_Add` (`self.MyArchList`) _asbp_arch_base)
  (`KismetSystemLibrary.PrintString` "Add"))

(fn `UserConstructionScript`)