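; Base weapon Blueprint that tracks ammo and fire rate and provides hitscan helpers, with a placeholder Fire function that only prints.
; IsFire gates shots on a BP_Time interval timer and remaining bullets, while WeaponFire restamps the timer and decrements ammo.
; ServerFire forwards to Fire; Onebullet separately line-traces on Visibility for BP_MyFPSMoveItCharacter hits.
; Reload refills to MaxBullets; the ServerDamage and WeaponReload events are empty.
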(event `ServerFire`
  (params (pos :type "Vector Structure") (vec :type "Vector Structure") (parent :type "/Game/Blueprints/BP_MyFPSMoveItCharacter Object Reference"))
  (`KismetSystemLibrary.PrintString` "----------------------------------------------oya")
  (`self.Fire` pos vec parent))

(event `ServerDamage`)

(event `Weapon Reload`)

(event `WeaponFire`
  (`/Game/Blueprints/BP_Time.SetNowTime` (`self.shotTimer`))
  (bind _result (`/Engine/EditorBlueprintResources/StandardMacros.DecrementInt` (`self.remainingBullets`))
    (:`  `
      (bind _output_get (set `self.remainingBullets` _result))
      (`KismetSystemLibrary.PrintString` (`KismetStringLibrary.Conv_IntToString` _output_get)))))

(event `self.ReceiveBeginPlay`
  (bind _returnvalue (`|GenericCreateObject` "/Game/Blueprints/BP_Time.BP_Time_C" self))
  (bind _output_get (set `self.shotTimer` _returnvalue))
  (`/Game/Blueprints/BP_Time.Init` _output_get)
  (set `self.remainingBullets` (`self.MaxBullets`)))

(event `self.ReceiveTick`
  (params (DeltaSeconds :type "Float (single-precision)")))

(fn `Fire`
  (params (pos :type "Vector Structure") (vec :type "Vector Structure") (parent :type "/Game/Blueprints/BP_MyFPSMoveItCharacter Object Reference"))
  (`KismetSystemLibrary.PrintString` "親Fire"))

(fn `isFire`
  (returns (isfire :type Boolean))
  (bind _milliseconds (`/Game/Blueprints/BP_Time.TimeSpan_milliseconds` (`self.shotTimer`)))
  (return (and (>= _milliseconds (`self.interval_millisecond`)) (> (`self.remainingBullets`) 0))))

(fn `isRemaining`
  (returns (isRemaining :type Boolean))
  (return (== (`self.MaxBullets`) (`self.remainingBullets`))))

(fn `Onebullet`
  (params (pos :type "Vector Structure") (vec :type "Vector Structure") (parent :type "/Game/Blueprints/BP_MyFPSMoveItCharacter Object Reference"))
  (returns (hit :type Boolean) (HitActor :type "Actor Object Reference"))
  (bind (_start _end) (`self.tracevec` pos vec 15000.0))
  (bind _outhit (`KismetSystemLibrary.LineTraceSingle` _start _end "TraceTypeQuery1" false (`|MakeArray` parent :!type "Actor Object Reference")))
  (bind (_bblockinghit _binitialoverlap _time _distance _location _impactpoint _normal _impactnormal _physmat _hitactor) (`GameplayStatics.BreakHitResult` _outhit))
  (return (and _bblockinghit (== (`GameplayStatics.GetObjectClass` _hitactor) "/Game/Blueprints/BP_MyFPSMoveItCharacter.BP_MyFPSMoveItCharacter_C")) _hitactor))

(fn `Reload`
  (set `self.remainingBullets` (`self.MaxBullets`)))

(fn `Set Weapon Anim Rate`
  (params (rate :type "Float (double-precision) (by ref)"))
  (if (== rate 0.0)
    (`SkeletalMeshComponent.SetPlayRate` (`self.WeaponMesh`) 1.0)
    (else
      (`SkeletalMeshComponent.SetPlayRate` (`self.WeaponMesh`) rate))))

(fn `tracevec`
  (params (pos :type "Vector Structure") (vec :type "Vector Structure") (mag :type "Float (double-precision)"))
  (returns (start :type "Vector Structure") (end :type "Vector Structure"))
  (return pos (+ pos (* vec mag))))

(fn `UserConstructionScript`)