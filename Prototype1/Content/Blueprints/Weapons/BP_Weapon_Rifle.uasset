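; Rifle weapon Blueprint, a child of a parent weapon class that supplies the fire and reload logic.
; It overrides WeaponFire and WeaponReload to call the parent, then play the matching rifle animation once on WeaponMesh.
; Reload uses a prone reload animation in every case, and the construction script and Tick only pass through to the parent.
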(event `self.Weapon Reload`
  (`parent.Weapon Reload`)
  (`SkeletalMeshComponent.PlayAnimation` (`self.WeaponMesh`) "/Game/MilitaryWeapSilver/Weapons/Animations/Prone_Reload_Rifle_W.Prone_Reload_Rifle_W" false))

(event `self.WeaponFire`
  (`parent.WeaponFire`)
  (`SkeletalMeshComponent.PlayAnimation` (`self.WeaponMesh`) "/Game/MilitaryWeapSilver/Weapons/Animations/Fire_Rifle_W.Fire_Rifle_W" false))

(event `self.ReceiveTick`
  (params (DeltaSeconds :type "Float (single-precision)"))
  (`parent.ReceiveTick` DeltaSeconds))

(fn `UserConstructionScript`
  (`parent.UserConstructionScript`))