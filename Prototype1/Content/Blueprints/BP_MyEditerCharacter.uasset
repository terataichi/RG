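; BP_MyEditerCharacter is the player character for editing a BP_MyStageMain stage by placing and taking.
; On BeginPlay it sends MyID to every BP_AddPlayer implementer through server-named events.
; Each Tick, a long eye-view line trace caches any stage hit in a RepNotify variable and passes the impact point to draw a space box.
; Put and Take inputs forward MyID to that cached stage; LineNoHit resets it but has no caller here.
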(event `self.ReceiveBeginPlay`
  (`self.InitMyIDServer`))

(event `InitMyIDServer`
  ;[1 1 1] イベント処理
  (bind _outactors (`GameplayStatics.GetAllActorsWithInterface` "/Game/Stage/BP/BP_AddPlayer.BP_AddPlayer_C"))
  (for _array_element _outactors
    (message `/Game/Stage/BP/BP_AddPlayer.AddPlayer` _array_element (`self.MyID`))))

(event `self.ReceiveTick`
  (params (DeltaSeconds :type "Float (single-precision)"))
  (bind (_outlocation _outrotation) (`self.GetActorEyesViewPoint`))
  (bind _outhit (`KismetSystemLibrary.LineTraceSingle` _outlocation (+ _outlocation (* (`KismetMathLibrary.Conv_RotatorToVector` _outrotation) 15000.0)) "TraceTypeQuery3"))
  (bind (_bblockinghit _binitialoverlap _time _distance _location _impactpoint _normal _impactnormal _physmat _hitactor) (`GameplayStatics.BreakHitResult` _outhit))
  (if _bblockinghit
    (bind _asbp_my_stage_main (cast `/Game/Stage/BP/BP_MyStageMain` _hitactor))
    (bind _output_get (set `self.As BP My Stage Main` _asbp_my_stage_main))
    (`self.DrawSpaceBoxServer` _output_get _impactpoint)))

(event `PutAction`
  (bind _as_bp_my_stage_main (`self.As BP My Stage Main`))
  ;[1 1 1] イベント処理
  (if (`KismetSystemLibrary.IsValid` _as_bp_my_stage_main)
    (`/Game/Stage/BP/BP_MyStageMain.PutServer` _as_bp_my_stage_main (`self.MyID`))))

(event `InputAction|Put`
  (params (Key :type "Key Structure"))
  (:`Pressed`
    (`self.PutAction`)))

(event `TakeAction`
  (bind _as_bp_my_stage_main (`self.As BP My Stage Main`))
  ;[1 1 1] イベント処理
  (if (`KismetSystemLibrary.IsValid` _as_bp_my_stage_main)
    (`/Game/Stage/BP/BP_MyStageMain.TakeServer` _as_bp_my_stage_main (`self.MyID`))))

(event `InputAction|Take`
  (params (Key :type "Key Structure"))
  (:`Pressed`
    (`self.TakeAction`)))

(event `DrawSpaceBoxServer`
  (params (StageMain :type "/Game/Stage/BP/BP_MyStageMain Object Reference (by ref)") (ImpactPoint :type "Vector Structure (by ref)"))
  ;[1 1 1] イベント処理
  (`/Game/Stage/BP/BP_MyStageMain.DrawSpaceSever` StageMain (`self.MyID`) ImpactPoint))

(event `LineNoHit`
  (bind _as_bp_my_stage_main (`self.As BP My Stage Main`))
  ;[1 1 1] イベント処理
  (if (`KismetSystemLibrary.IsValid` _as_bp_my_stage_main)
    (`/Game/Stage/BP/BP_MyStageMain.ResetServer` _as_bp_my_stage_main (`self.MyID`))))

(fn `OnRep_As BP My Stage Main`)

(fn `UserConstructionScript`)