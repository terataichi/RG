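; BP_MyFPSCharacter is an FPS character Blueprint with hold-to-sprint, rifle equipping and automatic fire.
; Left Shift doubles walk speed until released, and the 1 key spawns a rifle attached to a socket on the first-person mesh.
; While Fire is held, an axis event checks the weapon's interval against the shot timer and calls ServerFire; BP_ServerFire runs Fire.
; Tick prints the shot timer's milliseconds for debugging.
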(event `self.ReceiveTick`
  (params (DeltaSeconds :type "Float (single-precision)"))
  (bind _milliseconds (`/Game/Blueprints/BP_MyTime.TimeSpan_milliseconds` (`self.shotTime`)))
  (`KismetSystemLibrary.PrintString` (`KismetStringLibrary.Conv_DoubleToString` _milliseconds)))

(event `Key|LeftShift`
  (params (Key :type "Key Structure"))
  (bind _charactermovement (`self.CharacterMovement`))
  (bind _maxwalkspeed (`CharacterMovementComponent.MaxWalkSpeed` _charactermovement))
  ;[1 1 1] 最大移動スピード変更
  (:`Pressed`
    (set `self.savewalkspeed` _maxwalkspeed)
    (set `CharacterMovementComponent.MaxWalkSpeed` (* _maxwalkspeed 2.0) _charactermovement))
  (:`Released`
    (set `CharacterMovementComponent.MaxWalkSpeed` (`self.savewalkspeed`) _charactermovement)))

(event `Key|One`
  (params (Key :type "Key Structure"))
  ;[1 1 1] 武器を装備
  (:`Pressed`
    (bind _returnvalue (`|SpawnActorFromClass` "/Game/Blueprints/Weapons/BP_Weapon_Rifle.BP_Weapon_Rifle_C" (`self.GetTransform`) "Undefined" "OverrideRootScale" null null))
    (bind _output_get (set `self.myweapon_` _returnvalue))
    (`SceneComponent.K2_AttachToComponent` (`Actor.RootComponent` _output_get) (`self.FPSMesh`) "S_RifleSocket" "SnapToTarget" "SnapToTarget" "SnapToTarget" true)))

(event `InputAxis|FireKeep`
  (params (AxisValue :type "Float (single-precision)"))
  ;[1 1 1] 弾を発射
  (if (`self.isfire`)
    (bind _asbp_weapon_base (cast `/Game/Blueprints/Weapons/BP_WeaponBase` (`self.myweapon_`))
      (:`then`
        (bind _milliseconds (`/Game/Blueprints/BP_MyTime.TimeSpan_milliseconds` (`self.shotTime`)))
        (if (>= _milliseconds (`/Game/Blueprints/Weapons/BP_WeaponBase.interval_millisecond` _asbp_weapon_base))
          (set `self.shotTime` (`KismetMathLibrary.Now`))
          (`self.BP_ServerFire`)))
      (:`CastFailed`
        (`KismetSystemLibrary.PrintString` "アタッチされた武器無し")))))

(event `InputAction|Fire`
  (params (Key :type "Key Structure"))
  ;[1 1 1] 弾を発射
  (:`Pressed`
    (set `self.isfire` true))
  (:`Released`
    (set `self.isfire` false)))

(event `BP_ServerFire`
  ;[1 1 1] 弾を発射
  ;;[1 1 1] サーバーで実行
  (`self.Fire`))

(event `self.ReceiveBeginPlay`
  (`self.ServerBeginPlay`)
  (set `self.shotTime` (`KismetMathLibrary.Now`)))

(event `ServerBeginPlay`)

(event `self.ReceiveActorBeginOverlap`
  (params (OtherActor :type "Actor Object Reference")))

(fn `UserConstructionScript`)