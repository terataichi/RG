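; Player controller that manages a battle character and a spawned editor character (BP_MyEditerCharacter).
; Init enables component replication on both, hides the editor character without collision and attaches it to the battle one.
; SwapPlayer detaches two given characters and shows the first while hiding the second, toggling mesh visibility and collision.
; Its re-attach and Possess steps are unconnected, so control never actually transfers.
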(event `self.ReceiveBeginPlay`)

(fn `Init`
  (params (Character :type "Character Object Reference (by ref)"))
  (bind _output_get (set `self.Battle` Character))
  (`self.ReplicatedInit` _output_get)
  (bind _returnvalue (`|SpawnActorFromClass` "/Game/Blueprints/BP_MyEditerCharacter.BP_MyEditerCharacter_C" (`KismetMathLibrary.MakeTransform` (0.0 0.0 0.0)) "AlwaysSpawn" "OverrideRootScale" null null))
  (bind _output_get_2 (set `self.Edit` _returnvalue))
  (`self.ReplicatedInit` _output_get_2)
  (`self.SetCharacterVisiblityandCollision` false _output_get_2)
  (`self.K2_SetActorTransform` (`self.Edit`) (`self.GetTransform` (`self.Battle`)) false true)
  (`self.K2_AttachToActor` (`self.Edit`) (`self.Battle`) "None" "KeepWorld" "KeepWorld" "KeepWorld" true)
  (`KismetSystemLibrary.PrintString` "controller" true true (struct :`G` 0.66 :`B` 1.0 :`A` 1.0) 100.0))

(fn `OnRep_Battle`)

(fn `ReplicatedInit`
  (params (charactor :type "Character Object Reference (by ref)"))
  (`ActorComponent.SetIsReplicated` (`Character.CharacterMovement` charactor) true)
  (`ActorComponent.SetIsReplicated` (`Character.CapsuleComponent` charactor) true)
  (`ActorComponent.SetIsReplicated` (`Character.Mesh` charactor) true)
  (return))

(fn `SetCharacterVisiblityandCollision`
  (params (visibility_and_Collision :type Boolean) (target :type "Character Object Reference (by ref)"))
  (locals (targetChar :type "Character Object Reference"))
  (bind _targetchar (`local.targetChar`))
  (bind _targetchar_2 (`local.targetChar`))
  (set `local.targetChar` target)
  (if visibility_and_Collision
    ;[1 1 1] 見えるようにする
    (`SceneComponent.SetVisibility` (`Character.Mesh` _targetchar_2) true false)
    (`PrimitiveComponent.SetCollisionEnabled` (`Character.CapsuleComponent` _targetchar_2) "QueryAndPhysics")
    (`PrimitiveComponent.SetCollisionEnabled` (`Character.Mesh` _targetchar_2) "QueryOnly")
    (else
      ;[1 1 1] 見えなくして、当たり判定も消す
      (`SceneComponent.SetVisibility` (`Character.Mesh` _targetchar) false false)
      (`PrimitiveComponent.SetCollisionEnabled` (`Character.CapsuleComponent` _targetchar) "NoCollision")
      (`PrimitiveComponent.SetCollisionEnabled` (`Character.Mesh` _targetchar) "NoCollision"))))

(fn `SwapPlayer`
  (params (chara1 :type "Character Object Reference (by ref)") (Chara2 :type "Character Object Reference (by ref)"))
  (locals (LChara1 :type "Character Object Reference") (LChara2 :type "Character Object Reference"))
  (set `local.LChara1` chara1)
  (set `local.LChara2` Chara2)
  (`self.K2_DetachFromActor` (`local.LChara1`) "KeepWorld" "KeepWorld" "KeepWorld")
  (`self.K2_DetachFromActor` (`local.LChara2`) "KeepWorld" "KeepWorld" "KeepWorld")
  (`self.SetCharacterVisiblityandCollision` false (`local.LChara2`))
  (`self.SetCharacterVisiblityandCollision` true (`local.LChara1`)))

(fn `UserConstructionScript`)