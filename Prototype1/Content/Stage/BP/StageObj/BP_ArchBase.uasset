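; BP_ArchBase is a stage object, apparently a base for arches, that can be shown, hidden or moved vertically.
; Sweep stores the current location and full bounds height, then SweepServer plays a timeline that offsets Z by that height times the track value.
; ChengeHiddnAndCollision sets visibility and collision, propagating to children only when hiding.
; NumPad 5 triggers Sweep, Tick prints the location, and Init is empty.
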(event `self.ReceiveTick`
  (params (DeltaSeconds :type "Float (single-precision)"))
  (`KismetSystemLibrary.PrintString` (`KismetStringLibrary.Conv_VectorToString` (`self.K2_GetActorLocation`))))

(event `ChengeHiddnAndCollision`
  (params (newHidden :type Boolean) (NewCollision :type Boolean))
  (`SceneComponent.SetHiddenInGame` (`self.DefaultSceneRoot`) newHidden newHidden)
  (`self.SetActorEnableCollision` NewCollision))

(event `Key|NumPadFive` :consume false
  (params (Key :type "Key Structure"))
  (:`Pressed`
    (`self.Sweep`)))

(event `SweepServer`
  (bind (_direction `_新規track_0`) (`Timeline|SweepLine`)
    (:`Update`
      (`self.K2_SetActorLocation` (`KismetMathLibrary.MakeVector` (.x (`self.NowPos`)) (.y (`self.NowPos`)) (+ (.z (`self.NowPos`)) (* `_新規track_0` (`self.GoalPos`))))))))

(fn `Init`)

(fn `Sweep`
  (set `self.GoalPos` (* 2 (.z (`.BoxExtent` (`self.GetActorBounds` false)))))
  (set `self.NowPos` (`self.K2_GetActorLocation`))
  (`self.SweepServer`))

(fn `UserConstructionScript`)