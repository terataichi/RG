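; BP_Flag is a team flag actor that characters can carry, drop and reset to its spawn spot.
; On begin play it saves its location and tints the cube through a dynamic material using its Color.
; Overlapping a BP_MyFPSMoveItCharacter snaps it to that character's FlagPoint, gated by a hard-coded "Red" Team check.
; Drop detaches it in place, while Reset detaches and teleports it home, both through Server-named events.
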(event `self.ReceiveBeginPlay`
  (`self.ServerInit`))

(event `ServerInit`
  (bind _cube (`self.Cube`))
  (set `self.InitPos` (`self.K2_GetActorLocation`))
  (bind _returnvalue (`PrimitiveComponent.CreateDynamicMaterialInstance` _cube 0 "/Game/Resorce/MyMate/Material/M_red_Light_Inst.M_red_Light_Inst" "M_red_Light"))
  (`PrimitiveComponent.SetMaterial` _cube 0 _returnvalue)
  (`MaterialInstanceDynamic.SetVectorParameterValue` _returnvalue "color" (`self.Color`)))

(event `self.ReceiveActorBeginOverlap`
  (params (OtherActor :type "Actor Object Reference"))
  (`self.CheckEnemyTeamAndAttach` OtherActor))

(event `CheckEnemyTeamAndAttach`
  (params (Actor :type "Actor Object Reference"))
  (bind _asbp_my_fpsmove_it_character (cast `/Game/Blueprints/BP_MyFPSMoveItCharacter` Actor))
  ;[1 1 1] チーム情報をみる
  (if (`KismetStringLibrary.EqualEqual_StrStr` (`self.Team`) "Red")
    ;[1 1 1] アタッチ
    (`self.K2_AttachToComponent` (`/Game/Blueprints/BP_MyFPSMoveItCharacter.FlagPoint` _asbp_my_fpsmove_it_character) "None" "SnapToTarget" "SnapToTarget" "SnapToTarget")))

(event `DetachServer`
  (`self.K2_DetachFromActor` "KeepWorld" "KeepWorld" "KeepWorld"))

(event `InitLocationServer`
  (`self.K2_SetActorLocation` (`self.InitPos`) false true))

(fn `Drop`
  (`self.DetachServer`))

(fn `Reset`
  (`self.DetachServer`)
  (`self.InitLocationServer`))

(fn `UserConstructionScript`)