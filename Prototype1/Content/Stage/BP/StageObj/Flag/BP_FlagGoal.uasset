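; BP_FlagGoal is a team-specific goal stage object that resets a matching team's flag when it reaches the goal.
; On BeginPlay, InitServer gives the Cube a dynamic red-light material instance and tints it with the Color variable.
; On actor overlap, CheckGoal casts the actor to BP_Flag and calls its Reset if both Team values match.
; No scoring happens in this Blueprint.
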(event `self.ReceiveBeginPlay`
  (`self.InitServer`))

(event `InitServer`
  (bind _cube (`self.Cube`))
  (bind _returnvalue (`PrimitiveComponent.CreateDynamicMaterialInstance` _cube 0 "/Game/Resorce/MyMate/Material/M_red_Light_Inst.M_red_Light_Inst" "M_red_Light"))
  (`PrimitiveComponent.SetMaterial` _cube 0 _returnvalue)
  (`MaterialInstanceDynamic.SetVectorParameterValue` _returnvalue "color" (`self.Color`)))

(event `self.ReceiveActorBeginOverlap`
  (params (OtherActor :type "Actor Object Reference"))
  (`self.CheckGoal` OtherActor))

(event `CheckGoal`
  (params (Actor :type "Actor Object Reference"))
  (bind _asbp_flag (cast `/Game/Stage/BP/StageObj/Flag/BP_Flag` Actor))
  ;[1 1 1] チーム情報をみる
  (if (`KismetStringLibrary.EqualEqual_StrStr` (`self.Team`) (`/Game/Stage/BP/StageObj/Flag/BP_Flag.Team` _asbp_flag))
    ;[1 1 1] Detach
    (`/Game/Stage/BP/StageObj/Flag/BP_Flag.Reset` _asbp_flag)))

(fn `UserConstructionScript`)