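; PortalBP is a stage portal that teleports an MICharacter overlapping its capsule to DesPos, offset 200 units along the player's facing direction.
; BeginPlay searches PortalSet actors for an uninitialized partner portal, but the pairing code that swaps locations and sets Init on both is disconnected and never runs.
; Every tick, the Portal component turns to face the player camera, with pitch held at zero.
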(event `self.ReceiveBeginPlay`
  ;[1 1 1] 相方のポータルを探す
  (if (not (`self.Init`))
    (bind _outactors (`GameplayStatics.GetAllActorsWithInterface` "/Game/Stage/BP/StageObj/PortalSet.PortalSet_C"))
    (for _array_element _outactors
      (if (!= _array_element self)
        (bind _asportal_bp (cast `/Game/Stage/BP/StageObj/PortalBP` _array_element))
        (if (not (`/Game/Stage/BP/StageObj/PortalBP.Init` _asportal_bp))
          _)))))

(event `self.Capsule.OnComponentBeginOverlap`
  (params (OverlappedComponent :type "PrimitiveComponent Object Reference") (OtherActor :type "Actor Object Reference") (OtherComp :type "PrimitiveComponent Object Reference") (OtherBodyIndex :type Integer) (bFromSweep :type Boolean) (SweepResult :type "HitResult Structure (by ref)"))
  ;[1 1 1] 当たってきたのがPlayerならワープ
  (bind _asmicharacter (cast `MICharacter` OtherActor))
  (`self.PlayerWarp` _asmicharacter))

(event `self.ReceiveTick`
  (params (DeltaSeconds :type "Float (single-precision)"))
  (bind _returnvalue (`GameplayStatics.GetPlayerCameraManager` 0))
  ;[1 1 1] 常にPlayerのほうを向く
  (if (`KismetSystemLibrary.IsValid` _returnvalue)
    (`SceneComponent.K2_SetWorldRotation` (`self.Portal`) (`KismetMathLibrary.MakeRotator` (.roll (`KismetMathLibrary.FindLookAtRotation` (`SceneComponent.K2_GetComponentLocation` (`self.Portal`)) (`PlayerCameraManager.GetCameraLocation` _returnvalue))) 0.0 (.yaw (`KismetMathLibrary.FindLookAtRotation` (`SceneComponent.K2_GetComponentLocation` (`self.Portal`)) (`PlayerCameraManager.GetCameraLocation` _returnvalue)))) false false)))

(event `PlayerWarp`
  (params (Player :type "MICharacter Object Reference (by ref)"))
  ;[1 1 1] ワープさせる処理
  (`self.K2_SetActorLocation` Player (+ (`self.DesPos`) (* (`KismetMathLibrary.Conv_RotatorToVector` (`self.K2_GetActorRotation` Player)) 200.0)) false true))

(fn `UserConstructionScript`)